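; Interactable toilet that the player character can sit on or leave, provided they carry paper; otherwise a dialogue message is requested.
; A collision overlap enables input and opens a gate for interaction.
; Sitting blends the view to the toilet, starts a Delay-looped spring arm rotation, plays a fart sound and notifies the game instance unless already used.
; Mouse axes feed either seated pitch/yaw for a clamped camera or normal character look.
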(event `Rotate Camera`
  (`SceneComponent.K2_AddRelativeRotation` (`self.SpringArm`) (`KismetMathLibrary.MakeRotator` 0.0 0.0 (* (`self.RotationSpeed`) 0.1)) false false)
  (`KismetSystemLibrary.Delay` 0.001)
  (`self.Rotate Camera`))

(event `InputAxis|Look Up / Down Mouse`
  (params (AxisValue :type "Float (single-precision)"))
  (bind _char_ref (`self.Char REF`))
  ;[0.005208 0.005208 0.005208] Pitch
  (if (`/Game/PlayerCharacter/Blueprints/BP_Character.onToilet` _char_ref)
    (bind _output_get (set `self.Pitch` (+ (`self.Pitch`) AxisValue)))
    (else
      (`Pawn.AddControllerPitchInput` _char_ref AxisValue))))

(event `Move camera`
  ;[0 0 0] Move Camera
  (if (`/Game/PlayerCharacter/Blueprints/BP_Character.onToilet` (`self.Char REF`))
    (`SceneComponent.K2_SetRelativeRotation` (`self.Camera`) (`KismetMathLibrary.MakeRotator` 0.0 (`KismetMathLibrary.FClamp` (* (stale `InputAxis|Look Up / Down Mouse` _output_get) -1.0) -90.0 90.0) (`KismetMathLibrary.FClamp` (stale `InputAxis|Turn Right / Left Mouse` _output_get) -90.0 90.0)) false false)
    (`KismetSystemLibrary.Delay` 0.001)
    (`self.Move camera`)))

(event `self.ReceiveBeginPlay`
  (bind _class (`|LoadAssetClass` (`self.CharREF`))
    (:`then`
      _)
    (:`Completed`
      _))
  (bind _asactor (castclass `Actor` _class)
    (:`then`
      _)
    (:`CastFailed`
      _))
  (bind _outactors (`GameplayStatics.GetAllActorsOfClass` _asactor)))

(event `EnhancedInput|/Game/PlayerCharacter/Input/Actions/IA_Interact`
  (params (ActionValue :type "Vector2D Structure") (ElapsedSeconds :type "Float (double-precision)") (TriggeredSeconds :type "Float (double-precision)") (InputAction :type "InputAction Object Reference" :default "/Game/PlayerCharacter/Input/Actions/IA_Interact.IA_Interact"))
  (bind _char_ref (`self.Char REF`))
  ;[1 1 1] Checks if the player has the paper of the count
  (:`Started`
    (if (> (`/Game/PlayerCharacter/Blueprints/BP_Character.Paper Count` (stale `self.Collision.OnComponentBeginOverlap` _asbp_character)) 0)
      (`/Engine/EditorBlueprintResources/StandardMacros.Gate` true :!label _label
        (:`Exit`
          (if (`/Game/PlayerCharacter/Blueprints/BP_Character.onToilet` _char_ref)
            (`/Game/PlayerCharacter/Blueprints/BP_Character.NotSatOnToilet` _char_ref)
            (else
              (`/Game/PlayerCharacter/Blueprints/BP_Character.SatOnToilet` _char_ref)
              (`|ExecutionSequence`
                (:`then_0`
                  (`PlayerController.SetViewTargetWithBlend` (`GameplayStatics.GetPlayerController` 0) self 0.5 "VTBlend_Linear" 0.0 false)
                  (`self.Rotate Camera`))
                (:`then_1`
                  (`KismetSystemLibrary.Delay` 0.2)
                  (`GameplayStatics.PlaySound2D` "/Game/Nathan/Sounds/FartStuff/Fart_Cue.Fart_Cue" 1.0 1.0 0.0 null null)
                  (if (not (`self.hasshit`))
                    (bind _asgi_shitzing (cast `/Game/gav/gi_shitzing` (`GameplayStatics.GetGameInstance`)))
                    (`/Game/gav/gi_shitzing.Shtsetting` _asgi_shitzing))
                  (`self.EnableInput` (`GameplayStatics.GetPlayerController` 0) :!label _label_2)
                  (goto _label :!via `Open`)))))))
      (else
        (message `/Game/Nathan/Interfaces/BPI_CharInfo.GetShowDialogue` (stale `self.ReceiveBeginPlay` _outactors) (`self.DialogueCantShit`))))))

(event `InputAxis|Turn Right / Left Mouse`
  (params (AxisValue :type "Float (single-precision)"))
  (bind _char_ref (`self.Char REF`))
  ;[0.01562 0.01562 0.01562] Yaw
  (if (`/Game/PlayerCharacter/Blueprints/BP_Character.onToilet` _char_ref)
    (bind _output_get (set `self.Yaw` (+ (`self.Yaw`) AxisValue)))
    (else
      (`Pawn.AddControllerYawInput` _char_ref (stale `InputAxis|Look Up / Down Mouse` AxisValue)))))

(event `self.Collision.OnComponentBeginOverlap`
  (params (OverlappedComponent :type "PrimitiveComponent Object Reference") (OtherActor :type "Actor Object Reference") (OtherComp :type "PrimitiveComponent Object Reference") (OtherBodyIndex :type Integer) (bFromSweep :type Boolean) (SweepResult :type "HitResult Structure (by ref)"))
  (bind _asbp_character (cast `/Game/PlayerCharacter/Blueprints/BP_Character` OtherActor))
  (set `self.Char REF` _asbp_character)
  (goto _label_2))

(event `self.Collision.OnComponentEndOverlap`
  (params (OverlappedComponent :type "PrimitiveComponent Object Reference") (OtherActor :type "Actor Object Reference") (OtherComp :type "PrimitiveComponent Object Reference") (OtherBodyIndex :type Integer))
  (cast `/Game/PlayerCharacter/Blueprints/BP_Character` OtherActor)
  (`self.DisableInput` (`GameplayStatics.GetPlayerController` 0))
  (goto _label :!via `Close`))

(event `/Game/DannyTheGoatButt/Blueprints/Interface/BPI_AI.HasPooed`
  (set `self.hasshit` true))

(fn `Get Patrol`
  (returns (`Patrol Route` :type "/Game/DannyTheGoatButt/Blueprints/AI/BP_PatrolPath Object Reference"))
  (return null))

(fn `UserConstructionScript`)