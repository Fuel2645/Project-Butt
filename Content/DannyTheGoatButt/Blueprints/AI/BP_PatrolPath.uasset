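; Patrol path for AI, built on a spline whose points serve as patrol stops.
; A function returns the world location of the spline point at the current index.
; An increment event steps that index by a direction value, reversing it at the last point.
; On returning to the first point, the direction becomes zero rather than positive, so further increments leave the index there.
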(event `Increment Patrol Index`
  (bind _output_get (set `self.Current Index` (+ (`self.Current Index`) (`self.Direction`))))
  (if (== _output_get (- (`SplineComponent.GetNumberOfSplinePoints` (`self.Spline`)) 1))
    (set `self.Direction` -1)
    (elif (== (`self.Current Index`) 0)
      (set `self.Direction` 0))))

(fn `Get Location Of Current Point`
  (returns (Location :type "Vector Structure"))
  (return (`SplineComponent.GetLocationAtSplinePoint` (`self.Spline`) (`self.Current Index`) "World")))

(fn `UserConstructionScript`)