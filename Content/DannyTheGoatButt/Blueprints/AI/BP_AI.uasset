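; AI employee character that patrols and reacts to seeing the player, driven by the BT_AI behavior tree started on possession.
; Perception sets CanSeePlayer; losing sight pauses the tree, moves to the last stimulus location, then restarts logic after a short delay.
; AddPatrol picks the nearest BP_PatrolPath, exposed through GetPatrol.
; DifferentModel rerolls to a different random employee mesh, and HasPooed sets a flag.
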(event `Different Model`
  (bind _mesh (`self.Mesh`))
  (bind _output_get (set `self.Random Mesh` (`KismetArrayLibrary.Array_Random` (`self.Employee Meshses`)) :!label _label))
  (if (!= _output_get (`SkinnedMeshComponent.SkeletalMesh` _mesh))
    (`SkeletalMeshComponent.SetSkeletalMeshAsset` _mesh (`self.Random Mesh`))
    (else
      (goto _label))))

(event `self.ReceivePossessed`
  (params (NewController :type "Controller Object Reference"))
  (bind _returnvalue (`AIBlueprintHelperLibrary.GetAIController` self))
  (`AIController.RunBehaviorTree` _returnvalue "/Game/DannyTheGoatButt/Blueprints/AI/BT_AI.BT_AI")
  (`BlackboardComponent.SetValueAsVector` (`AIBlueprintHelperLibrary.GetBlackboard` _returnvalue) "LastKnownLocation" (0.0 0.0 0.0)))

(event `self.AIPerception.OnTargetPerceptionUpdated`
  (params (Actor :type "Actor Object Reference") (Stimulus :type "AIStimulus Structure"))
  (bind _returnvalue (`AIBlueprintHelperLibrary.GetAIController` self))
  (bind _returnvalue_2 (`AIBlueprintHelperLibrary.GetBlackboard` _returnvalue))
  (bind _braincomponent (`AIController.BrainComponent` _returnvalue))
  (if (== Actor (`GameplayStatics.GetPlayerCharacter` 0))
    (if (`.bSuccessfullySensed` (break `AIStimulus` Stimulus))
      (`BlackboardComponent.SetValueAsBool` _returnvalue_2 "CanSeePlayer" true)
      (else
        (`BlackboardComponent.SetValueAsBool` _returnvalue_2 "CanSeePlayer" false)
        (`Controller.StopMovement` _returnvalue)
        (`BrainComponent.StopLogic` _braincomponent "")
        (`|AIMoveTo` self (`.StimulusLocation` (break `AIStimulus` Stimulus)) null
          (:`OnSuccess`
            _)
          (:`OnFail`
            _))
        (`KismetSystemLibrary.Delay` 1.0)
        (`BrainComponent.StartLogic` _braincomponent)))))

(event `Add Patrol`
  (bind _outactors (`GameplayStatics.GetAllActorsOfClass` "/Game/DannyTheGoatButt/Blueprints/AI/BP_PatrolPath.BP_PatrolPath_C"))
  (for _array_element _outactors
    (bind _returnvalue (`self.GetDistanceTo` _array_element self))
    (if (< _returnvalue (`self.Closest Distance`))
      (set `self.Closest Path` _array_element)
      (set `self.Closest Distance` _returnvalue)))
  (set `self.Patrol Path` (`self.Closest Path`)))

(event `/Game/DannyTheGoatButt/Blueprints/Interface/BPI_AI.HasPooed`
  (set `self.hasshit2` true))

(fn `Get Patrol`
  (returns (`Patrol Route` :type "/Game/DannyTheGoatButt/Blueprints/AI/BP_PatrolPath Object Reference"))
  (return (`self.Patrol Path`)))

(fn `UserConstructionScript`)