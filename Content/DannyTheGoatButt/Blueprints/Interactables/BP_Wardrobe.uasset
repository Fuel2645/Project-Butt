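; BP_Wardrobe is an interactable wardrobe whose first door swings open when used.
; On Interact with Door1, it stores the door's relative rotation, adds 120 degrees of yaw and lerps between them on the Rotate timeline.
; The lerped value is applied as world rotation, although the start is captured in relative space.
; Door1Open makes the opening one-way, and the Door2 branch does nothing.
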(event `/Game/Nathan/Interfaces/BPI_Interact.Interact`
  (params (Component :type "Object Object Reference"))
  (if (== Component (`self.Door 1`))
    (if (not (`self.Door 1 Open`))
      (bind _output_get (set `self.Start Rotation` (`SceneComponent.RelativeRotation` (`self.Door 1`))))
      (set `self.End Rotation` (`KismetMathLibrary.MakeRotator` (.roll _output_get) (.pitch _output_get) (+ (.yaw _output_get) 120.0)))
      (set `self.Door 1 Open` true)
      (bind (_direction _newtrack_0) (`Timeline|rotate` :!via `PlayFromStart`)
        (:`Update`
          (`SceneComponent.K2_SetWorldRotation` (`self.Door 1`) (`KismetMathLibrary.RLerp` (`self.Start Rotation`) (`self.End Rotation`) _newtrack_0) false false))))
    (elif (== Component (`self.Door 2`))
      _)))

(fn `UserConstructionScript`)